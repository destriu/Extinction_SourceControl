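; BP_Genass_Ballistic is a short-lived weapon projectile that deals damage to what it hits.
; It briefly disables collision on spawn, then enables it and self-destructs after just over a second.
; A hit destroys it, and a blocking hit first applies ProjectileDamage and spawns a plasma burst particle effect.
; The construction script tints both meshes pale yellow through a shared dynamic material instance.
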(event EventBeginPlay
  (Collision|SetCollisionEnabled "NoCollision")
  (Utilities|FlowControl|Delay 0.04)
  (Collision|SetCollisionEnabled "QueryAndPhysics")
  (Utilities|FlowControl|Delay 1.2)
  (Actor|DestroyActor))

(event Collision|EventHit
  (params (MyComp :type Primitive%20Component%20Object%20Reference) (Other :type Actor%20Object%20Reference) (OtherComp :type Primitive%20Component%20Object%20Reference) (bSelfMoved :type Boolean) (HitLocation :type Vector :default "0, 0, 0") (HitNormal :type Vector :default "0, 0, 0") (NormalImpulse :type Vector :default "0, 0, 0") (Hit :type Hit%20Result%20Structure%20%28by%20ref%29))
  (bind (_bblockinghit _binitialoverlap _time _location) (Collision|BreakHitResult Hit))
  (if _bblockinghit
    (Game|Damage|ApplyDamage Other (Variables|Default|GetProjectileDamage) 0 0)
    (Effects|SpawnEmitteratLocation "/Game/Characters/DasherSuit/DasherFX/FX_UWaveStarterKit/Particles/PAR_PlasmaBurst.PAR_PlasmaBurst" _location (Math|Rotator|Delta(Rotator) "0, 0, 0" (Transformation|GetWorldRotation)))
    (Actor|DestroyActor)
    (else
      (Actor|DestroyActor))))

(fn ConstructionScript
  (bind _returnvalue (Rendering|Material|CreateDynamicMaterialInstance "/Game/General_Materials/Particles/Bullet_Mat.Bullet_Mat" :!class /Script/Engine.KismetMaterialLibrary))
  (Variables|Default|SetDynamicMaterial _returnvalue)
  (Rendering|Material|SetVectorParameterValue (Variables|Default|GetDynamicMaterial) "GenassParticleColor" "(R=1.000000,G=0.924431,B=0.340000,A=1.000000)" :!class /Script/Engine.MaterialInstanceDynamic)
  (Rendering|Material|SetMaterial (Variables|Default|GetStaticMesh1) 0 (Variables|Default|GetDynamicMaterial)))